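; Base mission actor that tracks a staged delivery mission for the player's ship.
; On BeginPlay it loads mission data by MissionID from a data table and binds to the ship's objective-ID event.
; Each stage has one objective, completed by a single matching ID, which frees cargo space and shows a delivered widget.
; Completing a stage pays units, then loads the next objective's cargo or completes the mission in the ship's log.
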(event `self.ReceiveBeginPlay`
  (`self.getMissionDetails`)
  (add `/Game/Blueprints/BP_Ship.OnObjectiveID` (`/Game/CommonLibrary.GetShip`) (`|CreateDelegate` :!event `On Objective ID heard`)))

(fn `Complete Stage`
  (bind _ship (`/Game/CommonLibrary.GetShip`))
  (bind _ship_2 (`/Game/CommonLibrary.GetShip`))
  (set `/Game/Blueprints/BP_Ship.units` (+ (`/Game/Blueprints/BP_Ship.units` _ship) (`.Payout_7_C7F939354980D31926AEC297BD02CA91` (break `/Game/Missions/F_StageDetails` (`self.StageDetails`)))) _ship)
  (bind _output_get (set `self.CurrentStage` (+ (`self.CurrentStage`) 1)))
  (bind _output_get_2 (set `self.StageDetails` (`|GetArrayItem` (`.Stages_10_1D5BF49D491C6AF8388BADAFF467DB42` (break `/Game/Missions/F_MissionDetails` (`self.MissionDetails`))) _output_get)))
  (bind _returnvalue (`self.isMissionComplete`))
  (if _returnvalue
    (`/Game/UI/MissionLog.Complete` (`/Game/Blueprints/BP_Ship.MissionLog` (`/Game/CommonLibrary.GetShip`)) (`self.MissionID`) self)
    (else
      (`BlueprintMapLibrary.Map_Clear` (`self.ObjectiveProgress`))
      (bind (_name _objectiveid _location _size _additionalsize) (break `/Game/Missions/F_Objective` (`.Objective_13_C9F568154ACC8B43FDE142818D20EB90` (break `/Game/Missions/F_StageDetails` _output_get_2))))
      (`BlueprintMapLibrary.Map_Add` (`self.ObjectiveProgress`) _objectiveid)
      (set `/Game/Blueprints/BP_Ship.usedSpace` (+ (`/Game/Blueprints/BP_Ship.usedSpace` _ship_2) _additionalsize) _ship_2)
      (`/Game/UI/MissionLog.RedrawLog` (`/Game/Blueprints/BP_Ship.MissionLog` (`/Game/CommonLibrary.GetShip`))))))

(fn `getMissionDetails`
  (bind _returnvalue (`|GetDataTableRow` "/Game/Missions/NewDataTable.NewDataTable" (`self.MissionID`))
    (:`then`
      (bind _output_get (set `self.MissionDetails` _returnvalue))
      (bind (_missionname _loginfo _stages _totalstages _npctext _currentstage) (break `/Game/Missions/F_MissionDetails` _output_get))
      (set `self.CurrentStage` _currentstage)
      (bind _output_get_2 (set `self.StageDetails` (`|GetArrayItem` _stages _currentstage)))
      (`BlueprintMapLibrary.Map_Clear` (`self.ObjectiveProgress`))
      (`BlueprintMapLibrary.Map_Add` (`self.ObjectiveProgress`) (`.ObjectiveID_8_D0BF7AF54E4E9E54072C64A7826B8340` (break `/Game/Missions/F_Objective` (`.Objective_13_C9F568154ACC8B43FDE142818D20EB90` (break `/Game/Missions/F_StageDetails` _output_get_2))))))))

(fn `getObjectiveData`
  (params (`Objective ID` :type String))
  (returns (Objective :type "/Game/Missions/F_Objective Structure"))
  (bind (_stagename _desc _payout _objective) (break `/Game/Missions/F_StageDetails` (`self.StageDetails`)))
  (if (`KismetStringLibrary.EqualEqual_StrStr` (`.ObjectiveID_8_D0BF7AF54E4E9E54072C64A7826B8340` (break `/Game/Missions/F_Objective` _objective)) `Objective ID`)
    (return _objective)))

(fn `isMissionComplete`
  (returns (ReturnValue :type Boolean))
  (return (== (`.totalStages_21_8B600734487C78A568E219BC7BBCAB96` (break `/Game/Missions/F_MissionDetails` (`self.MissionDetails`))) (`self.CurrentStage`))))

(fn `isObjectiveComplete`
  (params (`Objective ID` :type String))
  (bind _ship (`/Game/CommonLibrary.GetShip`))
  (if (>= (`BlueprintMapLibrary.Map_Find` (`self.ObjectiveProgress`) (`local.Objective ID`)) 1)
    (set `/Game/Blueprints/BP_Ship.usedSpace` (- (`/Game/Blueprints/BP_Ship.usedSpace` _ship) (`.Size_17_C84874C74225976BE559CD9ED8D3FD40` (break `/Game/Missions/F_Objective` (`self.getObjectiveData` `Objective ID`)))) _ship)
    (bind _returnvalue (`|CreateWidget` "/Game/UI/WB_Delivered.WB_Delivered_C"))
    (`UserWidget.AddToViewport` _returnvalue 0)
    (`self.Complete Stage`)))

(fn `On Objective ID Heard`
  (params (ObjectiveID :type String))
  (bind _objectiveid (`local.ObjectiveID`))
  (bind (_value _returnvalue) (`BlueprintMapLibrary.Map_Find` (`self.ObjectiveProgress`) ObjectiveID))
  (if _returnvalue
    (if (< _value 1)
      (`BlueprintMapLibrary.Map_Add` (`self.ObjectiveProgress`) _objectiveid (+ _value 1))
      (`self.isObjectiveComplete` _objectiveid)
      (return))
    (else
      (return))))

(fn `UserConstructionScript`)