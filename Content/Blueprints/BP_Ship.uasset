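; Player-controlled physics ship Blueprint with flight controls and mission interaction.
; Axis inputs apply pitch, yaw and roll torques and ease Thrust into a forward velocity.
; TakeOff scales thruster lift by mass and tilt until Thrust reaches a threshold, then forward velocity overrides physics velocity.
; Box overlaps with mission-tagged components store a look-at actor, whose Interact result feeds CallOnObjectiveID; speed widget and center-of-mass setup are disconnected.
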(event `InputAxis|TakeOff`
  (params (AxisValue :type "Float (single-precision)"))
  (bind (_returnvalue_x _returnvalue_y _returnvalue_z) (`KismetMathLibrary.BreakVector` (`self.GetActorUpVector`)))
  (if (>= (`self.thrust`) 100.0)
    (`PrimitiveComponent.SetPhysicsLinearVelocity` (`self.Ship`) (`self.forwardVelocity`) false "None")
    (else
      (set `PhysicsThrusterComponent.ThrustStrength` (* (/ (* AxisValue 500.0) _returnvalue_z) (`PrimitiveComponent.GetMass` (`self.Ship`))) (`self.PhysicsThruster`)))))

(event `self.Box.OnComponentBeginOverlap`
  (params (OverlappedComponent :type "PrimitiveComponent Object Reference") (OtherActor :type "Actor Object Reference") (OtherComp :type "PrimitiveComponent Object Reference") (OtherBodyIndex :type Integer) (bFromSweep :type Boolean) (SweepResult :type "HitResult Structure (by ref)"))
  (if (`ActorComponent.ComponentHasTag` OtherComp "mission")
    (bind _output_get (set `self.Look at Actor` OtherActor))
    (message `/Game/Blueprints/I_Interaction.LookAt` _output_get)))

(event `self.ReceiveBeginPlay`
  (`KismetSystemLibrary.PrintString` (`KismetSystemLibrary.GetDisplayName` (`GameplayStatics.GetPlayerPawn` 0))))

(event `InputAction|Interact`
  (params (Key :type "Key Structure"))
  (:`Pressed`
    (bind _look_at_actor (`self.Look at Actor`)
      (:`then`
        (bind _objectiveid (message `/Game/Blueprints/I_Interaction.InteractWith` _look_at_actor))
        (`self.OnObjectiveID` _objectiveid))
      (:`else`))))

(event `InputAxis|MoveUp`
  (params (AxisValue :type "Float (single-precision)"))
  (`PrimitiveComponent.AddTorqueInDegrees` (`self.Ship`) (* (`SceneComponent.GetRightVector` (`self.Ship`)) (* AxisValue (`self.ForwardTorquePower`))) "None" true))

(event `InputAxis|MoveRight`
  (params (AxisValue :type "Float (single-precision)"))
  (`PrimitiveComponent.AddTorqueInDegrees` (`self.Ship`) (* (`SceneComponent.GetUpVector` (`self.Ship`)) (* AxisValue (`self.SideTorquePower`))) "None" true))

(event `InputAxis|Roll`
  (params (AxisValue :type "Float (single-precision)"))
  (`PrimitiveComponent.AddTorqueInDegrees` (`self.Ship`) (* (`SceneComponent.GetForwardVector` (`self.Ship`)) (* AxisValue (`self.RotateTorque`))) "None" true))

(event `InputAxis|Thrust`
  (params (AxisValue :type "Float (single-precision)"))
  (bind _returnvalue (* AxisValue 7.0))
  (`|ExecutionSequence`
    (:`then_0`
      (if (not (`KismetMathLibrary.NearlyEqual_FloatFloat` AxisValue 0.0 0.1))
        (set `self.thrust` (`KismetMathLibrary.FInterpTo` (`self.thrust`) (`KismetMathLibrary.Lerp` 0.0 (`self.maxThrust`) _returnvalue) (`GameplayStatics.GetWorldDeltaSeconds`) 0.1))
        (`KismetSystemLibrary.PrintString` (`KismetStringLibrary.Conv_DoubleToString` _returnvalue))))
    (:`then_1`
      (set `self.forwardVelocity` (* (`SceneComponent.GetForwardVector` (`self.Ship`)) (`self.thrust`))))))

(fn `UserConstructionScript`)