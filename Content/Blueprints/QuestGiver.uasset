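; Quest giver component that offers its owner's mission to the player on interaction.
; InteractWith checks the ship's MissionLog and prints a notice if the mission is already active.
; Otherwise, DisplayMission looks up the MissionData row handle in its data table and opens a WB_Mission widget with the details and row name as ID.
; Interaction returns the owner's display name either way, and the Lookat event is an empty stub.
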(event `/Game/Blueprints/I_Interaction.LookAt`)

(fn `DisplayMission`
  (bind (_missiondata_datatable _missiondata_rowname) (break `DataTableRowHandle` (`self.MissionData`)))
  (bind _returnvalue (`|GetDataTableRow` _missiondata_datatable _missiondata_rowname)
    (:`then`
      (bind _returnvalue_2 (`|CreateWidget` "/Game/UI/WB_Mission.WB_Mission_C" null _returnvalue _missiondata_rowname))
      (`UserWidget.AddToViewport` _returnvalue_2 0))))

(fn `InteractWith`
  (returns (ObjectiveID :type String))
  (bind (_missiondata_datatable _missiondata_rowname) (break `DataTableRowHandle` (`self.MissionData`)))
  (bind _returnvalue (`KismetSystemLibrary.GetDisplayName` (`self.GetOwner`)))
  (if (not (`/Game/UI/MissionLog.QueryActive` (`/Game/Blueprints/BP_Ship.MissionLog` (`/Game/CommonLibrary.GetShip`)) _missiondata_rowname))
    (`self.DisplayMission`)
    (return _returnvalue)
    (else
      (`KismetSystemLibrary.PrintString` "Already doing mission")
      (return _returnvalue))))